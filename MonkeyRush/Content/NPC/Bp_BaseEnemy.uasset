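; Base enemy Blueprint with health that hurts the main character on contact and is destroyed when its health runs out.
; Capsule overlap with BP_mainChar calls GetHurtedAndLaunch with OverlapDMG, unless the overlapping component is the player's attack box.
; Incoming damage reduces Health and attaches an explosion emitter to the Sprite.
; Death is polled every Tick, destroying the actor once Health reaches zero or below.
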(event `self.ReceiveActorBeginOverlap`
  (params (OtherActor :type "Actor Object Reference")))

(event `self.ReceiveTick`
  (params (DeltaSeconds :type "Float (single-precision)"))
  (`self.isDead?`))

(event `self.CapsuleComponent.OnComponentBeginOverlap`
  (params (OverlappedComponent :type "PrimitiveComponent Object Reference") (OtherActor :type "Actor Object Reference") (OtherComp :type "PrimitiveComponent Object Reference") (OtherBodyIndex :type Integer) (bFromSweep :type Boolean) (SweepResult :type "HitResult Structure (by ref)"))
  (bind _asbp_main_char (cast `/Game/Character/BP_mainChar` OtherActor))
  (if (not (== (`/Game/Character/BP_mainChar.AttackingBoxCollision` _asbp_main_char) OtherComp))
    (`/Game/Character/BP_mainChar.GetHurtedAndLaunch` _asbp_main_char (`self.OverlapDMG`))))

(event `self.ReceiveAnyDamage`
  (params (Damage :type "Float (single-precision)") (DamageType :type "DamageType Object Reference") (InstigatedBy :type "Controller Object Reference") (DamageCauser :type "Actor Object Reference"))
  (set `self.Health` (- (`self.Health`) (`KismetMathLibrary.FTrunc` Damage)))
  (`GameplayStatics.SpawnEmitterAttached` "/Game/StarterContent/Particles/P_Explosion.P_Explosion" (`self.Sprite`)))

(fn `UserConstructionScript`)