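; Neutral NPC that turns in yaw to face the player and shows line-by-line dialogue when interacted with.
; On BeginPlay it caches Dialogues data table row names matching its NPCID.
; Each interaction advances LineCurrent, finds the row for the current ConversationID and line, and shows it in WBP_NPC_Dialogue.
; Without exactly one match it closes the widget and resets the line; leaving the Box only closes the widget.
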(event `/Game/Interafces/Interact.Interact_i`
  (bind (_returnvalue_roll _returnvalue_pitch _returnvalue_yaw) (`KismetMathLibrary.BreakRotator` (`KismetMathLibrary.FindLookAtRotation` (`self.K2_GetActorLocation`) (`self.K2_GetActorLocation` (`GameplayStatics.GetPlayerCharacter` 0)))))
  ;[1 1 1] Act with a NPC, and turn to Character
  (`/Engine/EditorBlueprintResources/StandardMacros.IncrementInt` (`self.LineCurrent`)
    (:`  `
      (`self.DialogueCreate`)
      (`self.K2_SetActorRotation` (`KismetMathLibrary.MakeRotator` 0.0 0.0 _returnvalue_yaw)))))

(event `self.ReceiveBeginPlay`
  ;[1 1 1] Add Dialogue inex to array
  (bind _outrownames (`DataTableFunctionLibrary.GetDataTableRowNames` "/Game/NPC/Dialogues.Dialogues"))
  (for _array_element _outrownames
    (bind _returnvalue (`|GetDataTableRow` "/Game/NPC/Dialogues.Dialogues" _array_element)
      (:`then`
        (if (== (`.NPC_ID_5_E59B34FE48BF1B4968E13DBEEAC9ED07` (break `/Game/NPC/DialogueStruct` _returnvalue)) (`self.NPC_ID`))
          (`KismetArrayLibrary.Array_Add` (`self.MyDialogue`) _array_element))))))

(event `self.Box.OnComponentEndOverlap`
  (params (OverlappedComponent :type "PrimitiveComponent Object Reference") (OtherActor :type "Actor Object Reference") (OtherComp :type "PrimitiveComponent Object Reference") (OtherBodyIndex :type Integer))
  ;[1 1 1] Remove widget
  (cast `/Game/Character/BP_mainChar` OtherActor)
  (`Widget.RemoveFromParent` (`self.NPC_Dialogue_Widget`))
  (set `self.NPC_Dialogue_Widget` null))

(fn `DialogueCreate`
  (`/Engine/EditorBlueprintResources/StandardMacros.IsValid` (`self.NPC_Dialogue_Widget`)
    (:`Is Valid`
      (bind _returnline (`self.DialogueGetLine`))
      (set `/Game/Blueprints/HUD/WBP_NPC_Dialogue.DialogText` _returnline (`self.NPC_Dialogue_Widget`)))
    (:`Is Not Valid`
      (bind _returnvalue (`|CreateWidget` "/Game/Blueprints/HUD/WBP_NPC_Dialogue.WBP_NPC_Dialogue_C" (`GameplayStatics.GetPlayerController` 0)))
      (bind _output_get (set `self.NPC_Dialogue_Widget` _returnvalue))
      (`UserWidget.AddToViewport` _output_get 0)
      (bind _returnline_2 (`self.DialogueGetLine`))
      (set `/Game/Blueprints/HUD/WBP_NPC_Dialogue.DialogText` _returnline_2 (`self.NPC_Dialogue_Widget`)))))

(fn `DialogueGetLine`
  (returns (ReturnLine :type Text))
  (locals (Return_Lines :type "Array of Text"))
  (for _array_element (`self.MyDialogue`)
    (bind _returnvalue (`|GetDataTableRow` "/Game/NPC/Dialogues.Dialogues" _array_element)
      (:`then`
        (bind (_npc_id _conversation_id _line_id _dialogue) (break `/Game/NPC/DialogueStruct` _returnvalue))
        (if (and (== _conversation_id (`self.Conversation_ID`)) (== _line_id (`self.LineCurrent`)))
          (`KismetArrayLibrary.Array_Add` (`local.Return_Lines`) _dialogue)))))
  (if (== (`KismetArrayLibrary.Array_Length` (`local.Return_Lines`)) 1)
    (return (`|GetArrayItem` (`local.Return_Lines`)))
    (else
      (`Widget.RemoveFromParent` (`self.NPC_Dialogue_Widget`))
      (set `self.NPC_Dialogue_Widget` null)
      (set `self.LineCurrent` 0))))

(fn `UserConstructionScript`)