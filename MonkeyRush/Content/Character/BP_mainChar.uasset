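; Player character Blueprint that handles attack, spell cast and slide input and creates the player's UI widgets.
; Attack and cast halt movement, then restore walking after a delay; casting spends AbilitySystemComponent mana to spawn a test projectile, or plays a no-mana animation.
; Slide adds smoke and an X-axis impulse based on MovementRight, then stops after a brief delay.
; BeginPlay builds the HUD, stats and no-mana widgets; C toggles stats.
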(event `InputAction|AttackButton`
  (params (Key :type "Key Structure"))
  ;[1 1 1] Attacking
  (:`Pressed`
    (`MovementComponent.StopMovementImmediately` (`self.CharacterMovement`))
    (`self.StartAttacking`)
    (`KismetSystemLibrary.Delay` 3.0)
    (`CharacterMovementComponent.SetMovementMode` (`self.CharacterMovement`) "MOVE_Walking" 0)))

(event `InputAction|SpellCastButton`
  (params (Key :type "Key Structure"))
  (bind _abilitysystemcomponent (`self.AbilitySystemComponent`))
  (bind _nomanawidget (`self.NoManaWidget`))
  (bind _mana (`AbilitySystemComponent.Mana` _abilitysystemcomponent))
  ;[1 1 1] SpellCasting TODO: CAST SPELL Delay
  (:`Pressed`
    (if (>= _mana 5)
      (set `AbilitySystemComponent.Mana` (- _mana 5) _abilitysystemcomponent)
      (`MovementComponent.StopMovementImmediately` (`self.CharacterMovement`))
      (`self.StartCastingSpell`)
      (`KismetSystemLibrary.Delay` 0.2)
      (`CharacterMovementComponent.SetMovementMode` (`self.CharacterMovement`) "MOVE_Walking" 0)
      (`|SpawnActorFromClass` "/Game/Spells/MySpellProjectileTest.MySpellProjectileTest_C" (`self.GetTransform`) "Undefined" "OverrideRootScale" null null)
      (else
        (`UserWidget.PlayAnimation` _nomanawidget (`/Game/HUD/WBP_NoMana.ManaAnimation` _nomanawidget) 0.0 1 "Forward" 1.0)))))

(event `InputAction|SlideButton`
  (params (Key :type "Key Structure"))
  (bind _charactermovement (`self.CharacterMovement`))
  ;[1 1 1] Sliding
  (:`Pressed`
    (`GameplayStatics.SpawnEmitterAttached` "/Game/StarterContent/Particles/P_Smoke.P_Smoke" (`self.RootComponent`) "None" (0.0 0.0 0.0) (struct) (3.0 3.0 3.0))
    (`self.StartSliding`)
    (if (`self.bMovementRight`)
      (`CharacterMovementComponent.AddImpulse` _charactermovement (8000.0 0.0 0.0) true)
      (else
        (`CharacterMovementComponent.AddImpulse` _charactermovement (-8000.0 0.0 0.0) true)))
    (`KismetSystemLibrary.Delay` 0.2)
    (`MovementComponent.StopMovementImmediately` (`self.CharacterMovement`))))

(event `self.ReceiveBeginPlay`
  (`self.CreateWidgets`))

(event `Key|C`
  (params (Key :type "Key Structure"))
  ;[1 1 1] Set visibility stats widget
  (:`Pressed`
    (`/Engine/EditorBlueprintResources/StandardMacros.FlipFlop`
      (:`A`
        (`Widget.SetVisibility` (`self.StatsWidget`) "Visible"))
      (:`B`
        (`Widget.SetVisibility` (`self.StatsWidget`) "Collapsed")))))

(fn `UserConstructionScript`)