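; Quest dealer actor that handles the player's act button for stepping through dialog text.
; On an ActButton press while its Box reports an overlap, it increments TextIndex and tries to copy the value to a WBP_QuestDiealer_Dialog widget.
; The widget reference comes from casting the player controller to that widget class, so the copy stops at the failed cast.
; BeginPlay, overlap and Tick only call the parent.
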(event `self.ReceiveBeginPlay`
  (`parent.ReceiveBeginPlay`))

(event `self.ReceiveActorBeginOverlap`
  (params (OtherActor :type "Actor Object Reference"))
  (`parent.ReceiveActorBeginOverlap` OtherActor))

(event `self.ReceiveTick`
  (params (DeltaSeconds :type "Float (single-precision)"))
  (`parent.ReceiveTick` DeltaSeconds))

(event `InputAction|ActButton`
  (params (Key :type "Key Structure"))
  (:`Pressed`
    (if (`PrimitiveComponent.IsOverlappingActor` (`self.Box`) null)
      (bind _result (`/Engine/EditorBlueprintResources/StandardMacros.IncrementInt` (`self.TextIndex`))
        (:`  `
          (bind _aswbp_quest_diealer_dialog (cast `/Game/Blueprints/QuestDiealer/WBP_QuestDiealer_Dialog` (`GameplayStatics.GetPlayerController` 0)))
          (set `/Game/Blueprints/QuestDiealer/WBP_QuestDiealer_Dialog.TexxtIndex` _result _aswbp_quest_diealer_dialog))))))

(fn `UserConstructionScript`
  (`parent.UserConstructionScript`))